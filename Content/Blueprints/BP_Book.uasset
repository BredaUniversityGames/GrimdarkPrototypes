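; BP_Book is an interactable book actor that holds text with keyword slots and tracks whether its keywords have been collected.
; On BeginPlay it swaps numbered placeholders (keyword1, keyword2, etc.) for KeywordArray entries using substring splitting and FormatText, then prints the result on screen.
; SetInteractText shows or hides the TextRender prompt, and CollectKeywords only sets the WasCollected flag.
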(event `self.ReceiveBeginPlay`
  (bind _text (`self.Text`))
  (for (_array_element _array_index) (`self.KeywordArray`)
    (bind _returnvalue (`KismetTextLibrary.Conv_TextToString` (`|FormatText` "keyword{index}" (+ _array_index 1))))
    (bind _returnvalue_2 (`KismetStringLibrary.FindSubstring` _text _returnvalue false false 0))
    (bind _returnvalue_3 (+ _returnvalue_2 (`KismetStringLibrary.Len` _returnvalue)))
    (set `self.Text` (`KismetTextLibrary.Conv_TextToString` (`|FormatText` "{Text Before} {Keyword} {Text After}" (`KismetStringLibrary.GetSubstring` _text 0 _returnvalue_2) _array_element (`KismetStringLibrary.GetSubstring` _text _returnvalue_3 (- (`KismetStringLibrary.Len` (`self.Text`)) _returnvalue_3))))))
  (`KismetSystemLibrary.PrintString` (`self.Text`) true true (struct :`G` 0.66 :`B` 1.0 :`A` 1.0) 1000.0))

(event `Set Interact Text`
  (params (Hidden :type Boolean))
  (`SceneComponent.SetHiddenInGame` (`self.TextRender`) Hidden false))

(event `CollectKeywords`
  (set `self.WasCollected` true))

(fn `UserConstructionScript`)