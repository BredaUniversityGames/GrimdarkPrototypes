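; BP_CustomCharacter is a Character Blueprint that serves as a debug scratchpad for movement values.
; BeginPlay registers Variable through AddVariableToTrack, and Tick prints the frame's delta seconds to screen.
; Disconnected chains and loose nodes hold earlier probes of acceleration, velocity and max speed, including the only increment of Variable, so none of them run.
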(event `self.ReceiveBeginPlay`
  (`JumpVisualizationBPLibrary.AddVariableToTrack` (`self.Variable`)))

(event `self.ReceiveTick`
  (params (DeltaSeconds :type "Float (single-precision)"))
  (`KismetSystemLibrary.PrintString` (`KismetStringLibrary.Conv_DoubleToString` DeltaSeconds)))

(fn `UserConstructionScript`)